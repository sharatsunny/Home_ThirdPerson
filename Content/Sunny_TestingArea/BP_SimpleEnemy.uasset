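; BP_SimpleEnemy is a simple damageable test enemy that respawns in place after its health runs out.
; BeginPlay fills CurrentHP from MaxHP and caches the original static mesh.
; AnyDamage subtracts damage, and at zero or below it optionally spawns an emitter, clears the mesh, then restores mesh and health after a short Delay.
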(event EventBeginPlay
  (Variables|Default|SetCurrentHP (Variables|Default|GetMaxHP))
  (Variables|Default|SetOriginalSM (Variables|/Script/Engine.StaticMeshComponent|GetStaticMesh (Variables|Default|GetStaticMesh))))

(event Collision|EventActorBeginOverlap
  (params (OtherActor :type Actor%20Object%20Reference)))

(event EventTick
  (params (DeltaSeconds :type Float%20%28single-precision%29)))

(event Game|Damage|EventAnyDamage
  (params (Damage :type Float%20%28single-precision%29) (DamageType :type Damage%20Type%20Object%20Reference) (InstigatedBy :type Controller%20Object%20Reference) (DamageCauser :type Actor%20Object%20Reference))
  (bind _output_get (Variables|Default|SetCurrentHP (- (Variables|Default|GetCurrentHP) Damage)))
  (if (<= _output_get 0.0)
    (if (Variables|Default|GetSpawnEmitterOnDeath?)
      (Effects|SpawnEmitteratLocation (Variables|Default|GetEmitterToSpawn) (Transformation|GetActorLocation)))
    (Components|StaticMesh|SetStaticMesh (Variables|Default|GetStaticMesh) 0)
    (Utilities|FlowControl|Delay 2.0)
    (Components|StaticMesh|SetStaticMesh (Variables|Default|GetStaticMesh) (Variables|Default|GetOriginalSM))
    (Variables|Default|SetCurrentHP (Variables|Default|GetMaxHP))))

(fn ConstructionScript)