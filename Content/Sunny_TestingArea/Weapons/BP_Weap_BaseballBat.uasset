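; BP_Weap_BaseballBat is a baseball bat weapon that damages tagged targets.
; Its CheckApplyDamage event receives a target, checks that it is valid and carries AttackTag, then applies Damage to it.
; BeginPlay and the construction script only call the parent, the overlap event is disabled, and nothing in this graph triggers the damage check.
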(event Custom|CheckApplyDamage
  (params (Target :type Actor%20Object%20Reference))
  (Utilities|IsValid Target
    (:Is%20Valid
      (if (Actor|ActorHasTag Target (Variables|Default|GetAttackTag))
        (Game|Damage|ApplyDamage Target (Variables|Default|GetDamage) 0 0)))))

(event EventBeginPlay
  (|CallParentFunction))

(event Collision|EventActorBeginOverlap
  (params (OtherActor :type Actor%20Object%20Reference))
  (|CallParentFunction OtherActor) ; This node is disabled and will not be called.\nDrag off pins to build functionality.
)

(fn ConstructionScript
  (|CallParentFunction))